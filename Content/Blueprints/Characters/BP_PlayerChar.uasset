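; Player character Blueprint that uses the Gameplay Ability System for stats and skills, with world-axis movement input.
; On BeginPlay, if IsInit is set, it loads a data asset to initialize attributes from a DataTable, walk speed, identity, skills and AnimBP move/idle animations.
; It then prints attributes for debugging and grants only NormalSkill, which IA_Space activates by class.
; Activate and Deactivate are empty stubs, and ReadData leaves CardSkillGroup unfilled.
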(event Input|EnhancedActionEvents|EnhancedInputActionIA_Movement
  (params (ActionValue :type Vector%202D%20Structure) (ElapsedSeconds :type Float%20%28double-precision%29) (TriggeredSeconds :type Float%20%28double-precision%29) (InputAction :type Input%20Action%20Object%20Reference :default "/Game/Assets/Characters/PlayerChar/Input/IA_Movement.IA_Movement"))
  (bind (_x _y) (Math|Vector2D|BreakVector2D ActionValue))
  ;[0.15 0.15 0.15 0.5] move
  (Variables|Default|SetXDir _x)
  (Variables|Default|SetYDir _y)
  (Pawn|Input|AddMovementInput "1.000000,0.000000,0.000000" (Variables|Default|GetXDir) false)
  (Pawn|Input|AddMovementInput "0.000000,1.000000,0.000000" (Variables|Default|GetYDir) false))

(event Input|EnhancedActionEvents|EnhancedInputActionIA_Space
  (params (ActionValue :type Boolean) (ElapsedSeconds :type Float%20%28double-precision%29) (TriggeredSeconds :type Float%20%28double-precision%29) (InputAction :type Input%20Action%20Object%20Reference :default "/Game/Assets/Characters/PlayerChar/Input/IA_Space.IA_Space"))
  (Abilities|TryActivateAbilitybyClass (Variables|Default|GetAbilitySystemComp) (.Skill (Utilities|Struct|BreakSSkill (Variables|Skill|GetNormalSkill))) true))

(event EventBeginPlay
  (CallFunction|ReadData)
  (CallFunction|PrintAttribute)
  (CallFunction|GiveSkillGroup))

(event Collision|EventActorBeginOverlap
  (params (OtherActor :type Actor%20Object%20Reference)))

(event EventTick
  (params (DeltaSeconds :type Float%20%28single-precision%29)))

(fn ConstructionScript)

(fn Activate)

(fn Deactivate)

(fn ReadData
  (if (Variables|Default|GetIsInit)
    (bind (_dt_attribute _id _tag _name _icon _weight _normalskill _leftskill _rightskill _switchskill _moveanim _idleanim) (Default|ReadDataAsset (Variables|Attribute|GetDataAsset)))
    (CallFunction|SetData _dt_attribute _id _tag _name _icon _weight _normalskill _leftskill _rightskill _switchskill 0 _moveanim _idleanim)))

(fn SetData
  (params (DT%20Attribute :type Data%20Table%20Object%20Reference) (ID :type Integer) (Tag :type Gameplay%20Tag%20Structure) (Name :type Text) (Icon :type Texture%202D%20Object%20Reference) (Weight :type Float%20%28double-precision%29) (NormalSkill :type S%20Skill%20Structure) (LeftSkill :type S%20Skill%20Structure) (RightSkill :type S%20Skill%20Structure) (SwitchSkill :type S%20Skill%20Structure) (CardSkillGroup :type Array%20of%20S%20Skill%20Structures) (MoveAnim :type Paper%20ZD%20Anim%20Sequence%20Object%20Reference) (IdleAnim :type Paper%20ZD%20Anim%20Sequence%20Object%20Reference))
  (bind _output_get (Variables|Default|SetDT_Attribute DT%20Attribute))
  (Class|AbilitySystemComponent|InitStats (Variables|Default|GetAbilitySystemComp) "/Script/ProjectMR.BaseAttributeSet" _output_get)
  (CallFunction|SetSpeedtoCharMoveComp (.CurrentValue (Utilities|Struct|BreakGameplayAttributeData (Variables|/Script/ProjectMR.BaseAttributeSet|GetSpeed (Variables|Default|GetBaseAttributeSetComp)))))
  (Variables|Default|SetID ID)
  (Variables|Default|SetTag Tag)
  (Variables|Default|SetName Name)
  (Variables|Default|SetWeight Weight)
  (Variables|Default|SetIcon Icon)
  (Variables|Skill|SetNormalSkill NormalSkill)
  (Variables|Skill|SetLeftSkill LeftSkill)
  (Variables|Skill|SetRightSkill RightSkill)
  (Variables|Skill|SetSwitchSkill SwitchSkill)
  (Variables|Skill|SetCardSkillGroup CardSkillGroup)
  (bind _aspzdabp_player_char (Utilities|Casting|CastToPZDABP_PlayerChar (Class|PaperZDCharacter|GetAnimInstance)))
  (LocalVariables|SetPZDBP_PlayerChar _aspzdabp_player_char)
  (Variables|/Game/Assets/Characters/PlayerChar/PZDABP_PlayerChar.PZDABP_PlayerChar_C|SetMoveAnim (LocalVariables|GetPZDBP_PlayerChar) MoveAnim)
  (Variables|/Game/Assets/Characters/PlayerChar/PZDABP_PlayerChar.PZDABP_PlayerChar_C|SetIdleAnim (LocalVariables|GetPZDBP_PlayerChar) IdleAnim))

(fn SetSpeedtoCharMoveComp
  (params (MaxWalkSpeed :type Float%20%28single-precision%29))
  (Variables|/Script/Engine.CharacterMovementComponent|SetMaxWalkSpeed (Variables|Character|GetCharacterMovement) MaxWalkSpeed))

(fn PrintAttribute
  (bind _baseattributesetcomp (Variables|Default|GetBaseAttributeSetComp))
  (bind _attack (Variables|/Script/ProjectMR.BaseAttributeSet|GetAttack _baseattributesetcomp))
  (bind _maxhealth (Variables|/Script/ProjectMR.BaseAttributeSet|GetMaxHealth _baseattributesetcomp))
  (bind _speed (Variables|/Script/ProjectMR.BaseAttributeSet|GetSpeed _baseattributesetcomp))
  (bind _avoidrate (Variables|/Script/ProjectMR.BaseAttributeSet|GetAvoidRate _baseattributesetcomp))
  (bind _breakdefense (Variables|/Script/ProjectMR.BaseAttributeSet|GetBreakDefense _baseattributesetcomp))
  (bind _critdamage (Variables|/Script/ProjectMR.BaseAttributeSet|GetCritDamage _baseattributesetcomp))
  (bind _critrate (Variables|/Script/ProjectMR.BaseAttributeSet|GetCritRate _baseattributesetcomp))
  (bind _health (Variables|/Script/ProjectMR.BaseAttributeSet|GetHealth _baseattributesetcomp))
  (bind _defense (Variables|/Script/ProjectMR.BaseAttributeSet|GetDefense _baseattributesetcomp))
  (bind (_basevalue _currentvalue) (Utilities|Struct|BreakGameplayAttributeData _speed))
  (bind (_basevalue_2 _currentvalue_2) (Utilities|Struct|BreakGameplayAttributeData _attack))
  (bind (_basevalue_3 _currentvalue_3) (Utilities|Struct|BreakGameplayAttributeData _avoidrate))
  (bind (_basevalue_4 _currentvalue_4) (Utilities|Struct|BreakGameplayAttributeData _breakdefense))
  (bind (_basevalue_5 _currentvalue_5) (Utilities|Struct|BreakGameplayAttributeData _critdamage))
  (bind (_basevalue_6 _currentvalue_6) (Utilities|Struct|BreakGameplayAttributeData _critrate))
  (bind (_basevalue_7 _currentvalue_7) (Utilities|Struct|BreakGameplayAttributeData _defense))
  (bind (_basevalue_8 _currentvalue_8) (Utilities|Struct|BreakGameplayAttributeData _health))
  (bind (_basevalue_9 _currentvalue_9) (Utilities|Struct|BreakGameplayAttributeData _maxhealth))
  (Development|PrintString (Utilities|String|Append "Attack:" (Utilities|String|ToString(Float) _basevalue_2) " " (Utilities|String|ToString(Float) _currentvalue_2)))
  (Development|PrintString (Utilities|String|Append "AvoidRate:" (Utilities|String|ToString(Float) _basevalue_3) " " (Utilities|String|ToString(Float) _currentvalue_3)))
  (Development|PrintString (Utilities|String|Append "BreakDefense:" (Utilities|String|ToString(Float) _basevalue_4) " " (Utilities|String|ToString(Float) _currentvalue_4)))
  (Development|PrintString (Utilities|String|Append "CritDamage:" (Utilities|String|ToString(Float) _basevalue_5) " " (Utilities|String|ToString(Float) _currentvalue_5)))
  (Development|PrintString (Utilities|String|Append "CritRate:" (Utilities|String|ToString(Float) _basevalue_6) " " (Utilities|String|ToString(Float) _currentvalue_6)))
  (Development|PrintString (Utilities|String|Append "Defense:" (Utilities|String|ToString(Float) _basevalue_7) " " (Utilities|String|ToString(Float) _currentvalue_7)))
  (Development|PrintString (Utilities|String|Append "Health:" (Utilities|String|ToString(Float) _basevalue_8) " " (Utilities|String|ToString(Float) _currentvalue_8)))
  (Development|PrintString (Utilities|String|Append "MaxHealth:" (Utilities|String|ToString(Float) _basevalue_9) " " (Utilities|String|ToString(Float) _currentvalue_9)))
  (Development|PrintString (Utilities|String|Append "Speed:" (Utilities|String|ToString(Float) _basevalue) " " (Utilities|String|ToString(Float) _currentvalue))))

(fn GiveSkillGroup
  (bind _normalskill (Variables|Skill|GetNormalSkill))
  (bind (_tag _name _description _icon _level _maxlevel _skill) (Utilities|Struct|BreakSSkill _normalskill))
  (GameplayAbilities|GiveAbility (Variables|Default|GetAbilitySystemComp) _skill _level -1))