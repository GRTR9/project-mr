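; BP_ObjHandler is an object handler that spawns and tracks the player's characters.
; On BeginPlay it registers itself on the GameInstance, spawns a BP_PlayerChar at the first PlayerStart's location using the DA_Rei data asset, adds it to PlayerCharGroup and has player controller 0 possess it.
; The functions for generating, saving and reading all player character data are empty stubs.
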(event EventBeginPlay
  (Variables|/Game/Blueprints/BP_GameInstance.BP_GameInstance_C|SetObjHandler (CallFunction|GetGameInstance) self)
  (bind _outactors (Actor|GetAllActorsOfClass "/Script/Engine.PlayerStart"))
  (if (!= (Utilities|Array|Length _outactors) 0)
    (bind _returnvalue (Game|SpawnActorfromClass "/Game/Blueprints/BP_PlayerChar.BP_PlayerChar_C" (Math|Transform|MakeTransform (Transformation|GetActorLocation (Utilities|Array|Get(acopy) _outactors)) "0, 0, 0" "1.000000,1.000000,1.000000") "Undefined" "MultiplyWithRoot" 0 "/Game/Assets/Characters/PlayerChar/Rei/DA_Rei.DA_Rei" (Variables|Default|GetIsInit) 0))
    (Utilities|Array|Add (Variables|Default|GetPlayerCharGroup) _returnvalue)
    (Pawn|Possess (Game|GetPlayerController 0) _returnvalue)))

(fn ConstructionScript)

(fn GenAllPlayerChar)

(fn SaveAllPlayerCharData)

(fn ReadAllPlayerCharData)