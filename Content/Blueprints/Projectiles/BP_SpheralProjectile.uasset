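; A pooled 2D flipbook projectile with a spherical hit area, reused through Activate and Deactivate rather than spawning and destroying.
; Activate sets visuals, movement, combat stats, target tag and a lifetime timer.
; Sphere overlaps record each matching PaperZD character once in HitObjGroup, without applying damage here.
; Deactivate clears the flipbook and hit list, parks the actor off-map, switches state and disables tick.
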(event OnComponentBeginOverlap(Sphere)
  (params (OverlappedComponent :type Primitive%20Component%20Object%20Reference) (OtherActor :type Actor%20Object%20Reference) (OtherComp :type Primitive%20Component%20Object%20Reference) (OtherBodyIndex :type Integer) (bFromSweep :type Boolean) (SweepResult :type Hit%20Result%20Structure%20%28by%20ref%29))
  (bind _hitobjgroup (Variables|Default|GetHitObjGroup))
  (bind _asbase_paper_zdcharacter (Utilities|Casting|CastToBasePaperZDCharacter OtherActor))
  (if (GameplayTags|MatchesTag (Variables|/Script/ProjectMR.BasePaperZDCharacter|GetTag _asbase_paper_zdcharacter) (Variables|Default|GetTargerTag))
    (if (not (Utilities|Array|ContainsItem _hitobjgroup OtherActor))
      (Utilities|Array|Add _hitobjgroup OtherActor))))

(event EventBeginPlay)

(event Collision|EventActorBeginOverlap
  (params (OtherActor :type Actor%20Object%20Reference)))

(event EventTick
  (params (DeltaSeconds :type Float%20%28single-precision%29)))

(fn ConstructionScript)

(fn Activate
  (params (Flipbook :type Paper%20Flipbook%20Object%20Reference) (Damage :type Float%20%28double-precision%29) (BreakDefense :type Float%20%28double-precision%29) (CritRate :type Float%20%28double-precision%29) (CritDamage :type Float%20%28double-precision%29) (Impact :type Float%20%28double-precision%29) (Speed :type Vector) (Size :type Vector) (HitRange :type Vector) (TargerTag :type Gameplay%20Tag%20Structure) (IsDisappearOnHit :type Boolean) (Pos :type Vector) (LifeCycle :type Float%20%28double-precision%29))
  (Sprite|SetFlipbook (Variables|Default|GetPaperFlipbook) Flipbook)
  (Variables|Attribute|SetDamage Damage)
  (Variables|Attribute|SetBreakDefense BreakDefense)
  (Variables|Attribute|SetCritRate CritRate)
  (Variables|Attribute|SetCritDamage CritDamage)
  (Variables|Attribute|SetImpact Impact)
  (Variables|/Script/Engine.MovementComponent|SetVelocity (Variables|Default|GetProjectileMovement) Speed)
  (Transformation|SetWorldScale3D (Variables|Default|GetPaperFlipbook) Size)
  (Transformation|SetWorldScale3D (Variables|Default|GetSphere) HitRange)
  (Variables|Default|SetTargerTag TargerTag)
  (Variables|Default|SetIsDisappearOnHit IsDisappearOnHit)
  (Variables|Default|SetState "NewEnumerator0")
  (Actor|Tick|SetActorTickEnabled true)
  (Transformation|SetActorLocation Pos false false)
  (Utilities|Time|SetTimerbyFunctionName 0 "Deactivate" LifeCycle))

(fn Deactivate
  (if (Class|KismetSystemLibrary|TimerExists 0 "Deactivate")
    (Utilities|Time|ClearTimerbyFunctionName 0 "Deactivate"))
  (Sprite|SetFlipbook (Variables|Default|GetPaperFlipbook))
  (Transformation|SetActorLocation "10000.000000,10000.000000,-1000.000000" false false)
  (Variables|Default|SetState "NewEnumerator1")
  (Utilities|Array|Clear (Variables|Default|GetHitObjGroup))
  (Actor|Tick|SetActorTickEnabled false))