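; Player character Blueprint with PaperZD animation that moves on world X/Y from Enhanced Input and takes its stats from a data asset.
; On BeginPlay, if IsInit is set, ReadDataAsset passes the asset's values to SetData without resetting Hp.
; SetData stores combat stats, pickup range and skills (except LeftSkill), sets walk speed from Spd, and pushes move and idle animations to the anim instance.
; Activate and Deactivate are empty stubs.
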(event Input|EnhancedActionEvents|EnhancedInputActionIA_Movement
  (params (ActionValue :type Vector%202D%20Structure) (ElapsedSeconds :type Float%20%28double-precision%29) (TriggeredSeconds :type Float%20%28double-precision%29) (InputAction :type Input%20Action%20Object%20Reference :default "/Game/Assets/Characters/PlayerChar/Input/IA_Movement.IA_Movement"))
  (bind (_x _y) (Math|Vector2D|BreakVector2D ActionValue))
  ;[0.15 0.15 0.15 0.5] move
  (Variables|Default|SetXDir _x)
  (Variables|Default|SetYDir _y)
  (Pawn|Input|AddMovementInput "1.000000,0.000000,0.000000" (Variables|Default|GetXDir) false)
  (Pawn|Input|AddMovementInput "0.000000,1.000000,0.000000" (Variables|Default|GetYDir) false))

(event EventBeginPlay
  (if (Variables|Default|GetIsInit)
    (CallFunction|ReadDataAsset false)))

(event Collision|EventActorBeginOverlap
  (params (OtherActor :type Actor%20Object%20Reference)))

(event EventTick
  (params (DeltaSeconds :type Float%20%28single-precision%29)))

(fn ConstructionScript)

(fn Activate)

(fn Deactivate)

(fn ReadDataAsset
  (params (IsInit :type Boolean))
  (bind (_maxhp _atk _def _spd _agi _ct _ctdamage _kb _pickuprange _normalskill _leftskill _rightskill _moveanim _idleanim) (Default|ReadDataAsset (Variables|Attribute|GetDataAsset)))
  (CallFunction|SetData _maxhp _atk _def _spd _agi _ct _ctdamage _kb _pickuprange _normalskill _leftskill _rightskill 0 _moveanim _idleanim)
  (if IsInit
    (Variables|Attribute|SetHp (Variables|Attribute|GetMaxHp))))

(fn SetData
  (params (MaxHp :type Integer) (Atk :type Integer) (Def :type Integer) (Spd :type Float%20%28double-precision%29) (Agi :type Float%20%28double-precision%29) (Ct :type Float%20%28double-precision%29) (CtDamage :type Float%20%28double-precision%29) (Kb :type Integer) (PickupRange :type Float%20%28double-precision%29) (NormalSkill :type BP%20Skill%20Base%20Object%20Reference) (LeftSkill :type BP%20Skill%20Base%20Object%20Reference) (RightSkill :type BP%20Skill%20Base%20Object%20Reference) (CardSkillGroup :type Array%20of%20BP%20Skill%20Base%20Object%20References) (MoveAnim :type Paper%20ZD%20Anim%20Sequence%20Object%20Reference) (IdleAnim :type Paper%20ZD%20Anim%20Sequence%20Object%20Reference))
  (Variables|Attribute|SetMaxHp MaxHp)
  (Variables|Attribute|SetAtk Atk)
  (Variables|Attribute|SetDef Def)
  (bind _output_get (Variables|Attribute|SetSpd Spd))
  (Variables|/Script/Engine.CharacterMovementComponent|SetMaxWalkSpeed (Variables|Character|GetCharacterMovement) _output_get)
  (Variables|Attribute|SetAgi Agi)
  (Variables|Attribute|SetCt Ct)
  (Variables|Attribute|SetCtDamage CtDamage)
  (Variables|Attribute|SetKb Kb)
  (Variables|Skill|SetNormalSkill NormalSkill)
  (Variables|Attribute|SetPickupRange PickupRange)
  (Variables|Skill|SetRightSkill RightSkill)
  (Variables|Skill|SetCardSkillGroup CardSkillGroup)
  (bind _aspzdabp_player_char (Utilities|Casting|CastToPZDABP_PlayerChar (Class|PaperZDCharacter|GetAnimInstance)))
  (LocalVariables|SetPZDBP_PlayerChar _aspzdabp_player_char)
  (Variables|/Game/Assets/Characters/PlayerChar/PZDABP_PlayerChar.PZDABP_PlayerChar_C|SetMoveAnim (LocalVariables|GetPZDBP_PlayerChar) MoveAnim)
  (Variables|/Game/Assets/Characters/PlayerChar/PZDABP_PlayerChar.PZDABP_PlayerChar_C|SetIdleAnim (LocalVariables|GetPZDBP_PlayerChar) IdleAnim))