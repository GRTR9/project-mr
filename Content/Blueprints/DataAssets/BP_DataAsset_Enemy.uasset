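; BP_DataAsset_Enemy is a data asset that defines an enemy type, including whether it is a boss.
; It holds identity and display fields, an attribute table reference, weight, a normal skill plus three numbered skills, and move and idle animations.
; Its only function, ReadDataAsset, returns all these fields at once as separate outputs, with no other logic.
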(fn ReadDataAsset
  (return (Variables|Default|GetDT_Attribute) (Variables|Default|GetID) (Variables|Default|GetTag) (Variables|Default|GetName) (Variables|Default|GetIcon) (Variables|Default|GetWeight) (Variables|Skill|GetNormalSkill) (Variables|Skill|GetFirstSkill) (Variables|Skill|GetSecondSkill) (Variables|Skill|GetThirdSkill) (Variables|Default|GetMoveAnim) (Variables|Default|GetIdleAnim) (Variables|Default|GetIsBoss)))