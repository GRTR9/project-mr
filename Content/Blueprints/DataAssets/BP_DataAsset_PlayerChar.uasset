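; Player character data asset that holds a character's definition: attribute data, identity, icon, weight, skills and animations.
; Skills fill normal, left, right and switch slots, alongside move and idle animations.
; A single ReadDataAsset function returns every field at once as separate outputs, with no other logic.
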(fn ReadDataAsset
  (return (Variables|Default|GetDT_Attribute) (Variables|Default|GetID) (Variables|Default|GetTag) (Variables|Default|GetName) (Variables|Default|GetIcon) (Variables|Default|GetWeight) (Variables|Skill|GetNormalSkill) (Variables|Skill|GetLeftSkill) (Variables|Skill|GetRightSkill) (Variables|Skill|GetSwitchSkill) (Variables|Default|GetMoveAnim) (Variables|Default|GetIdleAnim)))